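; BP_BonusBase is a bonus actor that changes the game speed when the player character hits it.
; Each tick it moves along the world backward vector at the GameMode's BlocksSpeed, scaled by delta time and without sweeping.
; On Hit, a BP_Character triggers MultiplyGameSpeed on the GameMode with the bonus's GameSpeedRatio.
; The bonus then destroys itself, whatever actor it hit.
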(event EventBeginPlay)

(event EventTick
  (params (DeltaSeconds :type Float%20%28single-precision%29))
  (Transformation|SetActorLocation (+ (Transformation|GetActorLocation) (* (Class|KismetMathLibrary|VectorBackward) (* (Variables|/Game/BluePrints/BP_GameMode.BP_GameMode_C|GetBlocksSpeed (Variables|Default|GetGameMode)) (Utilities|Time|GetWorldDeltaSeconds)))) false false))

(event Collision|EventHit
  (params (MyComp :type Primitive%20Component%20Object%20Reference) (Other :type Actor%20Object%20Reference) (OtherComp :type Primitive%20Component%20Object%20Reference) (bSelfMoved :type Boolean) (HitLocation :type Vector :default "0, 0, 0") (HitNormal :type Vector :default "0, 0, 0") (NormalImpulse :type Vector :default "0, 0, 0") (Hit :type Hit%20Result%20Structure%20%28by%20ref%29))
  (Utilities|FlowControl|Sequence
    (:then_0
      (Utilities|Casting|CastToBP_Character Other)
      (Default|MultiplyGameSpeed (Variables|Default|GetGameMode) (Variables|Default|GetGameSpeedRatio)))
    (:then_1
      (Actor|DestroyActor))))

(fn ConstructionScript)