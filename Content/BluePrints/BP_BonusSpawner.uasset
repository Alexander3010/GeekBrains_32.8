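; BP_BonusSpawner continuously spawns random bonus actors during play at random intervals.
; On BeginPlay it caches BP_GameMode, then loops forever, waiting a random delay capped by the game mode's BonusMaxTimeInterval.
; Each cycle spawns a random entry from BonusClasses at a random Lines actor's transform and passes it the game mode.
; Spawns adjust for collisions and are skipped if still blocked.
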(event EventBeginPlay
  (bind _asbp_game_mode (Utilities|Casting|CastToBP_GameMode (Game|GetGameMode)))
  (Variables|Default|SetGameMode _asbp_game_mode)
  (Utilities|FlowControl|Delay (* (Math|Random|RandomFloat) (Variables|/Game/BluePrints/BP_GameMode.BP_GameMode_C|GetBonusMaxTimeInterval (Variables|Default|GetGameMode))) :!label _label)
  (Game|SpawnActorfromClass (.OutItem (Utilities|Array|Random (Variables|Default|GetBonusClasses))) (Transformation|GetActorTransform (.OutItem (Utilities|Array|Random (Variables|Default|GetLines)))) "AdjustIfPossibleButDontSpawnIfColliding" 0 (Variables|Default|GetGameMode) 0)
  (goto _label))

(fn ConstructionScript)