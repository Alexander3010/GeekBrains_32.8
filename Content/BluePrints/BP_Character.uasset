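; Player character for a lane-based game that jumps and hops between lines using touch swipes or test keys.
; Touch release picks the dominant swipe axis; swipe down does nothing.
; Hops change a clamped line index, and Tick slides the actor's Y toward that line at capped speed with sweep.
; Dead is gated by CanDie, spawns an explosion, notifies BP_GameMode and starts a timer.
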(event Custom|OnSwipeRight
  (CallFunction|HopRight))

(event Custom|OnSwipeUp
  (Character|Jump))

(event Custom|OnSwipeDown)

(event Custom|OnSwipeLeft
  (CallFunction|HopLeft))

(event EventBeginPlay
  (bind _asbp_game_mode (Utilities|Casting|CastToBP_GameMode (Game|GetGameMode)))
  (Variables|Default|SetGameMode _asbp_game_mode))

(event EventTick
  (params (DeltaSeconds :type Float%20%28single-precision%29))
  (CallFunction|MovetoCurrentLine DeltaSeconds))

(event Input|KeyboardEvents|A
  (params (Key :type Key%20Structure :default "None"))
  ;[1 1 1] Test
  (:Pressed
    (CallFunction|HopLeft)))

(event Input|KeyboardEvents|D
  (params (Key :type Key%20Structure :default "None"))
  ;[1 1 1] Test
  (:Pressed
    (CallFunction|HopRight)))

(event Input|KeyboardEvents|SpaceBar
  (params (Key :type Key%20Structure :default "None"))
  ;[1 1 1] Test
  (:Pressed
    (Character|Jump))
  (:Released
    (Character|StopJumping)))

(event Input|TouchEvents|InputTouch
  (params (Location :type Vector) (FingerIndex :type ETouchIndex%20Enum))
  (:Pressed
    (Variables|Touch|SetTouchStart2DVector Location))
  (:Released
    (bind _output_get (Variables|Touch|SetTouchSwipe2DVector (- Location (Variables|Touch|GetTouchStart2DVector))))
    (if (Math|Vector|NotEqual(Vector) _output_get "0, 0, 0" 1.0)
      (if (> (Math|Float|Absolute(Float) (.x (Variables|Touch|GetTouchSwipe2DVector))) (Math|Float|Absolute(Float) (.y (Variables|Touch|GetTouchSwipe2DVector))))
        (if (> (.x (Variables|Touch|GetTouchSwipe2DVector)) 0.0)
          (CallFunction|OnSwipeRight)
          (else
            (CallFunction|OnSwipeLeft)))
        (elif (> (.y (Variables|Touch|GetTouchSwipe2DVector)) 0.0)
          (CallFunction|OnSwipeDown)
          (else
            (CallFunction|OnSwipeUp)))))))

(fn ConstructionScript)

(fn MovetoCurrentLine
  (params (DeltaSeconds :type Float%20%28single-precision%29))
  (bind _output_get (LocalVariables|SetOffset (.y (- (Transformation|GetActorLocation (Utilities|Array|Get(acopy) (Variables|Default|GetLines) (Variables|Default|GetCurrentLineIndex))) (Transformation|GetActorLocation)))))
  (if (not (Math|Float|NearlyEqual(Float) _output_get 0.0 1e-06))
    (Utilities|FlowControl|Sequence
      (:then_0
        (LocalVariables|SetMaxDistancePerTick (* (Variables|Default|GetHorizontalSpeed) DeltaSeconds))
        (if (> (Math|Float|Absolute(Float) (LocalVariables|GetOffset)) (LocalVariables|GetMaxDistancePerTick))
          (LocalVariables|SetOffset (* (Math|Float|Sign(Float) (LocalVariables|GetOffset)) (LocalVariables|GetMaxDistancePerTick)))))
      (:then_1
        (Transformation|SetActorLocation (+ (Transformation|GetActorLocation) (Math|Vector|MakeVector 0.0 (LocalVariables|GetOffset) 0.0)) true false)))))

(fn HopRight
  (bind _result (Math|Integer|IncrementInt (Variables|Default|GetCurrentLineIndex))
    (:%20%20
      (Variables|Default|SetCurrentLineIndex (Math|Integer|Clamp(Integer) _result 0 (- (Utilities|Array|Length (Variables|Default|GetLines)) 1))))))

(fn HopLeft
  (bind _result (Math|Integer|DecrementInt (Variables|Default|GetCurrentLineIndex))
    (:%20%20
      (Variables|Default|SetCurrentLineIndex (Math|Integer|Clamp(Integer) _result 0 (- (Utilities|Array|Length (Variables|Default|GetLines)) 1))))))

(fn Dead
  (if (Variables|Default|GetCanDie)
    (Variables|Default|SetCanDie false)
    (Effects|SpawnEmitteratLocation "/Game/Effects/FX/Particles/P_Grenade_Explosion_Light.P_Grenade_Explosion_Light" (Transformation|GetActorLocation))
    (Default|OnDead (Variables|Default|GetGameMode))
    (Utilities|Time|SetTimerbyEvent (EventDispatchers|CreateEvent :!event AllowDeath) 1.0)))

(fn AllowDeath
  (Variables|Default|SetCanDie true))