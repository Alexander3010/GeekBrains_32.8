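; BP_GameMode is the game mode for a block-based game, tracking health, score and game speed.
; From BeginPlay it caches BP_Hud and runs a looping Delay that raises Score at a rate tied to BlocksSpeed.
; OnDead decrements Health and, at zero or below, shows game over on the HUD UI, then pauses after a short delay.
; MultiplyGameSpeed scales BlocksSpeed up by a ratio and shrinks SpawnMaxTimeInterval by the same ratio.
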(event Custom|OnDead
  (bind _result (Math|Integer|DecrementInt (Variables|Default|GetHealth))
    (:%20%20
      (if (<= _result 0)
        (Default|OnGameOver (Variables|/Game/BluePrints/BP_Hud.BP_Hud_C|GetUI (Variables|Default|GetBP_Hud)))
        (Utilities|FlowControl|Delay 0.5)
        (Game|SetGamePaused true)))))

(event EventBeginPlay
  (bind _asbp_hud (Utilities|Casting|CastToBP_Hud (HUD|GetHUD (Game|GetPlayerController 0))))
  (Variables|Default|SetBP_Hud _asbp_hud)
  ;[1 1 1] Score
  (Utilities|FlowControl|Delay (/ 1.0 (Variables|Default|GetBlocksSpeed)) :!label _label)
  (Math|Integer|IncrementInt (Variables|Default|GetScore)
    (:%20%20
      (goto _label))))

(event EventTick
  (params (DeltaSeconds :type Float%20%28single-precision%29)))

(fn ConstructionScript)

(fn MultiplyGameSpeed
  (params (Ratio :type Float%20%28single-precision%29))
  (Variables|Default|SetBlocksSpeed (* (Variables|Default|GetBlocksSpeed) Ratio))
  (Variables|Default|SetSpawnMaxTimeInterval (/ (Variables|Default|GetSpawnMaxTimeInterval) Ratio)))