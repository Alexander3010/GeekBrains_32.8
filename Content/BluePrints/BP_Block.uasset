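; BP_Block is a moving obstacle that slides backward along the world axis each tick at the game mode's BlocksSpeed, scaled by delta time.
; Three colliders notify an overlapping BP_Character to hop right, hop left or die.
; The block destroys itself when it overlaps a KillZVolume.
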(event OnComponentBeginOverlap(DeadCollider)
  (params (OverlappedComponent :type Primitive%20Component%20Object%20Reference) (OtherActor :type Actor%20Object%20Reference) (OtherComp :type Primitive%20Component%20Object%20Reference) (OtherBodyIndex :type Integer) (bFromSweep :type Boolean) (SweepResult :type Hit%20Result%20Structure%20%28by%20ref%29))
  (bind _asbp_character (Utilities|Casting|CastToBP_Character OtherActor))
  (Default|Dead _asbp_character))

(event OnComponentBeginOverlap(RightHopCollider)
  (params (OverlappedComponent :type Primitive%20Component%20Object%20Reference) (OtherActor :type Actor%20Object%20Reference) (OtherComp :type Primitive%20Component%20Object%20Reference) (OtherBodyIndex :type Integer) (bFromSweep :type Boolean) (SweepResult :type Hit%20Result%20Structure%20%28by%20ref%29))
  (bind _asbp_character (Utilities|Casting|CastToBP_Character OtherActor))
  (Default|HopRight _asbp_character))

(event OnComponentBeginOverlap(LeftHopCollider)
  (params (OverlappedComponent :type Primitive%20Component%20Object%20Reference) (OtherActor :type Actor%20Object%20Reference) (OtherComp :type Primitive%20Component%20Object%20Reference) (OtherBodyIndex :type Integer) (bFromSweep :type Boolean) (SweepResult :type Hit%20Result%20Structure%20%28by%20ref%29))
  (bind _asbp_character (Utilities|Casting|CastToBP_Character OtherActor))
  (Default|HopLeft _asbp_character))

(event EventTick
  (params (DeltaSeconds :type Float%20%28single-precision%29))
  (Transformation|SetActorLocation (+ (Transformation|GetActorLocation) (* (Class|KismetMathLibrary|VectorBackward) (* (Variables|/Game/BluePrints/BP_GameMode.BP_GameMode_C|GetBlocksSpeed (Variables|Default|GetGameMode)) (Utilities|Time|GetWorldDeltaSeconds)))) false false))

(event Collision|EventActorBeginOverlap
  (params (OtherActor :type Actor%20Object%20Reference))
  (Utilities|Casting|CastToKillZVolume OtherActor)
  (Actor|DestroyActor))

(fn ConstructionScript)